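; BP_EnemySpawner populates a tunnel with a random number of BP_Enemy actors.
; SpawnEnemies clears its list, spawns a random count scaled by MaxEnemiesPerTunnel, and returns the new enemies.
; RandomSingleLocation places each enemy at a random offset from the given origin, within a box ahead along +X and centred on Y and Z.
; The event graph is empty, so spawning runs only when SpawnEnemies is called.
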(event EventBeginPlay)

(event Collision|EventActorBeginOverlap
  (params (OtherActor :type Actor%20Object%20Reference)))

(event EventTick
  (params (DeltaSeconds :type Float%20%28single-precision%29)))

(fn ConstructionScript)

(fn SpawnEnemies
  (params (InitLocation :type Vector))
  (Utilities|Array|Clear (Variables|Default|GetGeneratedEnemies))
  (for _index (range 0 (Math|Float|Truncate (* (Math|Random|RandomFloat) (Variables|Default|GetMaxEnemiesPerTunnel))))
    (bind _targetlocation (CallFunction|RandomSingleLocation InitLocation))
    (bind _returnvalue (Game|SpawnActorfromClass "/Game/InfiniteMatrix/Blueprints/BP_Enemy.BP_Enemy_C" (Math|Transform|MakeTransform _targetlocation "0, 0, 0" "1.000000,1.000000,1.000000") "Undefined" "MultiplyWithRoot" 0 0))
    (Utilities|Array|Add (Variables|Default|GetGeneratedEnemies) _returnvalue))
  (return (Variables|Default|GetGeneratedEnemies)))

(fn RandomSingleLocation
  (params (InitLocation :type Vector))
  (return (+ InitLocation (Math|Vector|MakeVector (+ (* (Math|Random|RandomFloat) 2e+03) 2.5e+02) (+ (* (Math|Random|RandomFloat) 6.5e+02) -325.0) (+ (* (Math|Random|RandomFloat) 6.5e+02) -325.0)))))